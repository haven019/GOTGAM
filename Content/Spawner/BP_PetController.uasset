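; BP_PetController executes pet battle commands (attack, defence, run, swap, capture) on the current test slot of the FirstPersonGameMode PetS array.
; Attack uses two timelines to lerp the pet along a fixed offset and back.
; Run lifts the pet by timeline, destroys it and opens Fieldmap01.
; Defence, swap and capture are placeholders that spawn an explosion and print; every action increments the slot as test turn-passing.
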(event Custom|DepenceActFunc
  ;[1 1 1] 2. 방어버튼
  (bind _asfirst_person_game_mode (Utilities|Casting|CastToFirstPersonGameMode (Game|GetGameMode)))
  (Effects|SpawnEmitteratLocation "/Game/StarterContent/Particles/P_Explosion.P_Explosion" (Transformation|GetActorLocation (Utilities|Array|Get(acopy) (Variables|/Game/FirstPersonBP/Blueprints/FirstPersonGameMode.FirstPersonGameMode_C|GetPetS _asfirst_person_game_mode) (Variables|Default|GettestSlot))))
  (Development|PrintString "2. Depence Button is clicked")
  (CallFunction|TestNext))

(event Custom|ChangeActFunc
  ;[1 1 1] 4. 펫교환버튼
  (bind _asfirst_person_game_mode (Utilities|Casting|CastToFirstPersonGameMode (Game|GetGameMode)))
  (Effects|SpawnEmitteratLocation "/Game/StarterContent/Particles/P_Explosion.P_Explosion" (Transformation|GetActorLocation (Utilities|Array|Get(acopy) (Variables|/Game/FirstPersonBP/Blueprints/FirstPersonGameMode.FirstPersonGameMode_C|GetPetS _asfirst_person_game_mode) (Variables|Default|GettestSlot))))
  (Development|PrintString "4. Change Button is clicked")
  (CallFunction|TestNext))

(event Custom|CaptureActFunc
  ;[1 1 1] 5. 포획 버튼
  (bind _asfirst_person_game_mode (Utilities|Casting|CastToFirstPersonGameMode (Game|GetGameMode)))
  (Effects|SpawnEmitteratLocation "/Game/StarterContent/Particles/P_Explosion.P_Explosion" (Transformation|GetActorLocation (Utilities|Array|Get(acopy) (Variables|/Game/FirstPersonBP/Blueprints/FirstPersonGameMode.FirstPersonGameMode_C|GetPetS _asfirst_person_game_mode) (Variables|Default|GettestSlot))))
  (Development|PrintString "5. Capture Button is clicked")
  (CallFunction|TestNext))

(event Custom|testNext
  ;[1 1 1] 테스트용: 다음 슬롯 지정
  (Math|Integer|IncrementInt (Variables|Default|GettestSlot)))

(event Custom|AttackActFunc
  (bind _testslot (Variables|Default|GettestSlot))
  ;[1 1 1] 1. 공격버튼
  (bind _asfirst_person_game_mode (Utilities|Casting|CastToFirstPersonGameMode (Game|GetGameMode)))
  (Variables|Default|SetStartLocation (Transformation|GetActorLocation (Utilities|Array|Get(acopy) (Variables|/Game/FirstPersonBP/Blueprints/FirstPersonGameMode.FirstPersonGameMode_C|GetPetS _asfirst_person_game_mode) _testslot)))
  (bind _move (Timeline|타임라인_0 Play)
    (:Update
      (Transformation|SetWorldLocation (Variables|/Script/Engine.Actor|GetRootComponent (Utilities|Array|Get(acopy) (Variables|/Game/FirstPersonBP/Blueprints/FirstPersonGameMode.FirstPersonGameMode_C|GetPetS _asfirst_person_game_mode) _testslot)) (Math|Vector|Lerp(Vector) (Variables|Default|GetStartLocation) (+ (Variables|Default|GetStartLocation) "0,-705.000000, 0") _move) true false))
    (:Finished
      (bind _move_2 (Timeline|타임라인_1 Play)
        (:Update
          (Transformation|SetWorldLocation (Variables|/Script/Engine.Actor|GetRootComponent (Utilities|Array|Get(acopy) (Variables|/Game/FirstPersonBP/Blueprints/FirstPersonGameMode.FirstPersonGameMode_C|GetPetS _asfirst_person_game_mode) _testslot)) (Math|Vector|Lerp(Vector) (Transformation|GetActorLocation (Utilities|Array|Get(acopy) (Variables|/Game/FirstPersonBP/Blueprints/FirstPersonGameMode.FirstPersonGameMode_C|GetPetS _asfirst_person_game_mode) _testslot)) (Variables|Default|GetStartLocation) _move_2) false false))
        (:Finished
          (CallFunction|TestNext))))))

(event Custom|RunActFunc
  ;[1 1 1] 3. 도망버튼
  (bind _asfirst_person_game_mode (Utilities|Casting|CastToFirstPersonGameMode (Game|GetGameMode)))
  (bind _move (Timeline|타임라인_2 Play)
    (:Update
      (Transformation|SetWorldLocation (Variables|/Script/Engine.Actor|GetRootComponent (Utilities|Array|Get(acopy) (Variables|/Game/FirstPersonBP/Blueprints/FirstPersonGameMode.FirstPersonGameMode_C|GetPetS _asfirst_person_game_mode) (Variables|Default|GettestSlot))) (Math|Vector|Lerp(Vector) (Transformation|GetActorLocation (Utilities|Array|Get(acopy) (Variables|/Game/FirstPersonBP/Blueprints/FirstPersonGameMode.FirstPersonGameMode_C|GetPetS _asfirst_person_game_mode) (Variables|Default|GettestSlot))) (+ (Transformation|GetActorLocation (Utilities|Array|Get(acopy) (Variables|/Game/FirstPersonBP/Blueprints/FirstPersonGameMode.FirstPersonGameMode_C|GetPetS _asfirst_person_game_mode) (Variables|Default|GettestSlot))) "0,0.000000,100.000000") _move) true false)
      (Development|PrintString "Run..."))
    (:Finished
      (Actor|DestroyActor (Utilities|Array|Get(acopy) (Variables|/Game/FirstPersonBP/Blueprints/FirstPersonGameMode.FirstPersonGameMode_C|GetPetS _asfirst_person_game_mode) (Variables|Default|GettestSlot)))
      (Development|PrintString "Run Success!")
      (CallFunction|TestNext)
      (Game|OpenLevel(byName) "Fieldmap01"))))

(event EventBeginPlay
  (bind _asfirst_person_game_mode (Utilities|Casting|CastToFirstPersonGameMode (Game|GetGameMode)))
  (Development|PrintString (Utilities|GetDisplayName (Utilities|Array|Get(acopy) (Variables|/Game/FirstPersonBP/Blueprints/FirstPersonGameMode.FirstPersonGameMode_C|GetPetS _asfirst_person_game_mode) (Variables|Default|GettestSlot)))))

(event EventTick
  (params (DeltaSeconds :type Float%20%28single-precision%29)))

(fn ConstructionScript)